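; Cover simulation actor that spawns a BP_4_Inch_HE actor at its Arrow component's transform when start_sim fires.
; It implements usable-interface events that forward to BPContextSensitiveUsableComponent, with the calls crossed: used events call StopUsed and stop-used events call Used.
; The team getter returns 0, and the usable-data getter and construction script are empty.
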(event Custom|start_sim
  (Game|SpawnActorfromClass "/Game/PostScriptum/Vehicles/UK/4_Inch_Mortar/BP_4_Inch_HE.BP_4_Inch_HE_C" (Transformation|GetWorldTransform (Variables|Default|GetArrow)) "Undefined" 0 0))

(event EventBPonUsed
  (params (User :type Controller%20Object%20Reference))
  (Default|StopUsed (Variables|Default|GetBP_ContextSensitiveUsableComponent) User))

(event EventBPStopUsed
  (params (User :type Controller%20Object%20Reference))
  (Default|Used (Variables|Default|GetBP_ContextSensitiveUsableComponent) User))

(event EventServeronUsed
  (params (User :type Controller%20Object%20Reference))
  (Default|StopUsed (Variables|Default|GetBP_ContextSensitiveUsableComponent) User))

(event EventServerStopUsed
  (params (User :type Controller%20Object%20Reference))
  (Default|Used (Variables|Default|GetBP_ContextSensitiveUsableComponent) User))

(fn ConstructionScript)

(fn GetInterfaceTeam
  (return 0))

(fn GetUsableData
  (return ""))