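; Moving-target shooting range controller that runs timed or untimed training rounds with a score and countdown display.
; Events choose distance (100/200/300 or random), fixed or random speed, and round length.
; Repeat waits briefly, picks a random spawn point, and spawns the matching left/right target with a reference back to this actor.
; Tick updates remaining time; RepNotifies refresh the text displays and play a client-side sound when score is above zero.
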(event Custom|move_200
  (Variables|Default|Set200 true)
  (Variables|Default|Set300 false)
  (Variables|Default|Setrandom_range false))

(event Custom|timer
  (Variables|Default|Settimer_var false)
  (CallFunction|Destroy)
  (Utilities|FlowControl|Delay 0.5)
  (Actor|Tick|SetActorTickEnabled false))

(event Custom|move_rand
  (Variables|Default|Setrandom_range true)
  (Variables|Default|Set300 false)
  (Variables|Default|Set200 false))

(event Custom|timer60
  (bind _output_get (Variables|Default|Settimer_float 6e+01))
  (Variables|Default|Settime_remain _output_get)
  (Variables|Default|SetnoTimer_bool false))

(event Custom|fixed_speed
  (Variables|Default|Setfixed true))

(event Custom|rand_speed
  (Variables|Default|Setfixed false))

(event Custom|timer180
  (bind _output_get (Variables|Default|Settimer_float 1.8e+02))
  (Variables|Default|Settime_remain _output_get)
  (Variables|Default|SetnoTimer_bool false))

(event Custom|timer300
  (bind _output_get (Variables|Default|Settimer_float 3e+02))
  (Variables|Default|Settime_remain _output_get)
  (Variables|Default|SetnoTimer_bool false))

(event Custom|notimer
  (Variables|Default|SetnoTimer_bool true)
  (Variables|Default|Settime_remain 13.37))

(event Custom|Stop
  (CallFunction|Timer)
  (Utilities|Time|ClearandInvalidateTimerbyHandle (stale Custom|start _returnvalue))
  (Variables|Default|Settime_remain 0.0))

(event Custom|score_increment
  (Variables|Default|Setscore_int (+ (Variables|Default|Getscore_int) 1)))

(event Custom|move_100
  (Variables|Default|Set200 false)
  (Variables|Default|Set300 false)
  (Variables|Default|Setrandom_range false))

(event Custom|repeat
  (if (Variables|Default|Gettimer_var)
    (Utilities|FlowControl|Delay (Math|Random|RandomFloatinRange 0.2 0.4))
    (if (Variables|Default|Get200)
      (CallFunction|SelectSpawn (Variables|Default|GetLeft200) (Variables|Default|GetRight200))
      (elif (Variables|Default|Get300)
        (CallFunction|SelectSpawn (Variables|Default|GetLeft300) (Variables|Default|GetRight300))
        (elif (Variables|Default|Getrandom_range)
          (CallFunction|RandomSpawn (Variables|Default|GetLeft100) (Variables|Default|GetLeft200) (Variables|Default|GetRight100) (Variables|Default|GetRight200) (Variables|Default|GetLeft300) (Variables|Default|GetRight300))
          (else
            (CallFunction|SelectSpawn (Variables|Default|GetLeft100) (Variables|Default|GetRight100))))))))

(event Custom|movement
  (bind _right300 (Variables|Default|GetRight300))
  (bind _current_spawn (Variables|Default|Getcurrent%20spawn))
  (bind _right100 (Variables|Default|GetRight100))
  (bind _right200 (Variables|Default|GetRight200))
  (bind _returnvalue (== _current_spawn _right100))
  (bind _returnvalue_2 (== _current_spawn _right300))
  (bind _returnvalue_3 (== _right200 _current_spawn))
  (bind _returnvalue_4 (Math|Boolean|ORBoolean _returnvalue_3 _returnvalue _returnvalue_2))
  (if (Variables|Default|Getfixed)
    (if _returnvalue_4
      (bind _returnvalue_5 (Game|SpawnActorfromClass "/6ga_training/moving_target/BP_movingtarget_training_R_fixed.BP_movingtarget_training_R_fixed_C" (Transformation|GetWorldTransform (Variables|Default|Getcurrent%20spawn)) "AdjustIfPossibleButAlwaysSpawn" 0 0))
      (bind _output_get (Variables|Default|Setcurrent%20target _returnvalue_5))
      (bind _asbp_movingtarget_training_r_fixed (Utilities|Casting|CastToBP_movingtarget_training_R_fixed _output_get))
      (Variables|/6ga_training/moving_target/BP_movingtarget_training_R_fixed.BP_movingtarget_training_R_fixed_C|Setactor _asbp_movingtarget_training_r_fixed self)
      (Transformation|SetWorldRotation (Variables|/Script/Engine.Actor|GetRootComponent _asbp_movingtarget_training_r_fixed) "0,90.000000, 0" false false)
      (else
        (bind _returnvalue_6 (Game|SpawnActorfromClass "/6ga_training/moving_target/BP_movingtarget_training_left_Fixed.BP_movingtarget_training_left_Fixed_C" (Transformation|GetWorldTransform (Variables|Default|Getcurrent%20spawn)) "AdjustIfPossibleButAlwaysSpawn" 0 0))
        (bind _output_get_2 (Variables|Default|Setcurrent%20target _returnvalue_6))
        (bind _asbp_movingtarget_training_left_fixed (Utilities|Casting|CastToBP_movingtarget_training_left_Fixed _output_get_2))
        (Variables|/6ga_training/moving_target/BP_movingtarget_training_left_Fixed.BP_movingtarget_training_left_Fixed_C|Setactor _asbp_movingtarget_training_left_fixed self)
        (Transformation|SetWorldRotation (Variables|/Script/Engine.Actor|GetRootComponent _asbp_movingtarget_training_left_fixed) "0,90.000000, 0" false false)))
    (elif _returnvalue_4
      (bind _returnvalue_7 (Game|SpawnActorfromClass "/6ga_training/moving_target/BP_movingtarget_training_R.BP_movingtarget_training_R_C" (Transformation|GetWorldTransform (Variables|Default|Getcurrent%20spawn)) "AdjustIfPossibleButAlwaysSpawn" 0 0))
      (bind _output_get_3 (Variables|Default|Setcurrent%20target _returnvalue_7))
      (bind _asbp_movingtarget_training_r (Utilities|Casting|CastToBP_movingtarget_training_R _output_get_3))
      (Variables|/6ga_training/moving_target/BP_movingtarget_training_R.BP_movingtarget_training_R_C|Setactor _asbp_movingtarget_training_r self)
      (Transformation|SetWorldRotation (Variables|/Script/Engine.Actor|GetRootComponent _asbp_movingtarget_training_r) "0,90.000000,0.000000" false false)
      (else
        (bind _returnvalue_8 (Game|SpawnActorfromClass "/6ga_training/moving_target/BP_movingtarget_training_left.BP_movingtarget_training_left_C" (Transformation|GetWorldTransform (Variables|Default|Getcurrent%20spawn)) "AdjustIfPossibleButAlwaysSpawn" 0 0))
        (bind _output_get_4 (Variables|Default|Setcurrent%20target _returnvalue_8))
        (bind _asbp_movingtarget_training_left (Utilities|Casting|CastToBP_movingtarget_training_left _output_get_4))
        (Variables|/6ga_training/moving_target/BP_movingtarget_training_left.BP_movingtarget_training_left_C|Setactor _asbp_movingtarget_training_left self)
        (Transformation|SetWorldRotation (Variables|/Script/Engine.Actor|GetRootComponent _asbp_movingtarget_training_left) "0,90.000000,0.000000" false false)))))

(event Custom|update%20time
  (Variables|Default|Settime_remain (Utilities|Time|GetTimerRemainingTimebyHandle (stale Custom|start _returnvalue))))

(event Custom|destroy
  (Actor|DestroyActor (Variables|Default|Getcurrent%20target)))

(event Custom|move_300
  (Variables|Default|Set300 true)
  (Variables|Default|Set200 false)
  (Variables|Default|Setrandom_range false))

(event Custom|start
  (Actor|Tick|SetActorTickEnabled true)
  (Utilities|Time|ClearandInvalidateTimerbyHandle (stale _returnvalue))
  (CallFunction|Destroy)
  (Variables|Default|Setscore_int 0)
  (Variables|Default|Settimer_var true)
  (Rendering|SetVisibility (Variables|Default|Gettime) true false)
  (if (Variables|Default|GetnoTimer_bool)
    _
    (else
      (bind _returnvalue (Utilities|Time|SetTimerbyEvent (delegate Custom|timer) (Variables|Default|Gettimer_float)))))
  (CallFunction|Repeat))

(event EventTick
  (params (DeltaSeconds :type Float%20%28single-precision%29))
  (CallFunction|UpdateTime))

(event EventBPonUsed
  (params (User :type Controller%20Object%20Reference))
  (Default|StopUsed (Variables|Default|GetBP_ContextSensitiveUsableComponent) User))

(event EventBPStopUsed
  (params (User :type Controller%20Object%20Reference))
  (Default|Used (Variables|Default|GetBP_ContextSensitiveUsableComponent) User))

(event EventServeronUsed
  (params (User :type Controller%20Object%20Reference))
  (Default|StopUsed (Variables|Default|GetBP_ContextSensitiveUsableComponent) User))

(event EventServerStopUsed
  (params (User :type Controller%20Object%20Reference))
  (Default|Used (Variables|Default|GetBP_ContextSensitiveUsableComponent) User))

(fn ConstructionScript)

(fn OnRepScoreInt
  (if (> (Variables|Default|Getscore_int) 0)
    (Networking|SwitchHasAuthority
      (:Authority
        _)
      (:Remote
        (Audio|PlaySoundatLocation "/Game/Audio/Character/Wounded/1pHit/01/1P_hit1_03.1P_hit1_03" (Transformation|GetWorldLocation (Variables|Default|Getfence_metal_panel_small_metal)) "0, 0, 0" 1.0 1.0 0.0 "/Game/Audio/Attenuation/AssaultRifle/AssaultRifleMidAttenuation.AssaultRifleMidAttenuation" 0 0))))
  (Rendering|Components|TextRender|SetText (Variables|Default|Get0) (Utilities|Text|ToText(Integer) (Variables|Default|Getscore_int) false true 2 2)))

(fn OnRepTimeRemain
  (if (> (Variables|Default|Gettime_remain) 0.0)
    (Rendering|Components|TextRender|SetTextRenderColor (Variables|Default|Gettime) (Math|Color|MakeColor 0 0 0 255))
    (Rendering|Components|TextRender|SetText (Variables|Default|Gettime) (Utilities|Text|ToText(Float) (Variables|Default|Gettime_remain) "HalfToEven" false true 2 3 2 2))
    (else
      (Rendering|Components|TextRender|SetTextRenderColor (Variables|Default|Gettime) (Math|Color|MakeColor 0 0 255 255))
      (Rendering|Components|TextRender|SetText (Variables|Default|Gettime) (Variables|Default|Gettimes%20up)))))

(fn SelectSpawn
  (params (Spawn[0] :type Arrow%20Component%20Object%20Reference) (Spawn[1] :type Arrow%20Component%20Object%20Reference))
  (bind _array (Utilities|Array|MakeArray Spawn[0] Spawn[1]))
  (Variables|Default|Setcurrent%20spawn (Utilities|Array|Get(acopy) _array (Math|Random|RandomInteger (Utilities|Array|Length _array))))
  (CallFunction|Movement))

(fn RandomSpawn
  (params (Spawn[0] :type Arrow%20Component%20Object%20Reference) (Spawn[1] :type Arrow%20Component%20Object%20Reference) (Spawn[2] :type Arrow%20Component%20Object%20Reference) (Spawn[3] :type Arrow%20Component%20Object%20Reference) (Spawn[4] :type Arrow%20Component%20Object%20Reference) (Spawn[5] :type Arrow%20Component%20Object%20Reference))
  (bind _array (Utilities|Array|MakeArray Spawn[0] Spawn[1] Spawn[2] Spawn[3] Spawn[4] Spawn[5]))
  (Variables|Default|Setcurrent%20spawn (Utilities|Array|Get(acopy) _array (Math|Random|RandomInteger (Utilities|Array|Length _array))))
  (CallFunction|Movement))

(fn GetInterfaceTeam
  (return 0))

(fn GetUsableData
  (return ""))