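; Spawner actor that places an ambient bounding machine-gun actor at its Arrow component's location.
; MGspawn destroys any previous instance, spawns a new one from the arrow's location only, and destroys it after a 60-second delay.
; It also stubs a rearm-source interface as an effectively unlimited supply: rearm checks and ammo consumption always succeed, while ammo-update binding is unsupported.
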(event Custom|MG%20spawn
  (Actor|DestroyActor (stale _returnvalue))
  (bind _returnvalue (Game|SpawnActorfromClass "/6ga_training/BCT/bounding/BP_Ambient_MG_bounding.BP_Ambient_MG_bounding_C" (Math|Conversions|ToTransform(Vector) (Transformation|GetWorldLocation (Variables|Default|GetArrow))) "AlwaysSpawn" 0 0))
  (Utilities|FlowControl|Delay 6e+01)
  (Actor|DestroyActor _returnvalue))

(fn ConstructionScript)

(fn BindEventtoAmmoUpdated
  (params (Delegate :type Delegate%20%28by%20ref%29))
  (return false))

(fn CanRearmPawn
  (params (Rearmer :type Pawn%20Object%20Reference))
  (return true))

(fn CanRearmWeapon
  (params (Weapon :type SQ%20Equipable%20Item%20Object%20Reference))
  (return true))

(fn ConsumeAmmo
  (params (AmmoRequired :type Float%20%28single-precision%29))
  (return true))

(fn GetAmmo
  (return 1e+08))

(fn GetRearmNoAmmoString
  (return ""))

(fn GetRearmSuccessString
  (return ""))

(fn GetRearmType
  (return "MainOrEnvironment"))

(fn UnbindEventtoAmmoUpdated
  (params (Delegate :type Delegate%20%28by%20ref%29))
  (return false))