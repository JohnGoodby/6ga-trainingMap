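; Medic exercise spawner that places six bodies at unique random arrow points and runs a five-minute countdown.
; Each body gets a reference to the spawner; decrementing the count to zero pauses the timer, while timeout or reset destroys all Body2 and Crouch_BP actors.
; Tick updates remaining time, and RepNotify variables refresh the time and body-count text displays.
; It also implements rearm functions as an effectively unlimited ammo source.
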(event Custom|Spawn%20Body
  (bind _array (Variables|Default|Getarray))
  (Actor|Tick|SetActorTickEnabled true)
  (Variables|Default|Setbodies 6)
  (Variables|Default|Settime_remain 3e+02)
  (CallFunction|DestroyTargets)
  (for _array_element (Utilities|Array|MakeArray (Variables|Default|GetArrow) (Variables|Default|GetArrow1) (Variables|Default|GetArrow2) (Variables|Default|GetArrow3) (Variables|Default|GetArrow4) (Variables|Default|GetArrow5) (Variables|Default|GetArrow6) (Variables|Default|GetArrow7) (Variables|Default|GetArrow8) (Variables|Default|GetArrow9) (Variables|Default|GetArrow10) (Variables|Default|GetArrow11) (Variables|Default|GetArrow12) (Variables|Default|GetArrow13) (Variables|Default|GetArrow14) (Variables|Default|GetArrow15) (Variables|Default|GetArrow16) (Variables|Default|GetArrow17) (Variables|Default|GetArrow18) (Variables|Default|GetArrow19))
    (Utilities|Array|Add (Variables|Default|Getarray) _array_element))
  (for _index (range 0 5)
    (Variables|Default|SetSpawn%20Index (Math|Random|RandomInteger (Utilities|Array|Length _array)))
    (bind _returnvalue (Game|SpawnActorfromClass "/6ga_training/medic/body/body2.body2_C" (Transformation|GetWorldTransform (Utilities|Array|Get(acopy) _array (Variables|Default|GetSpawn%20Index))) "AdjustIfPossibleButAlwaysSpawn" 0 0))
    (Utilities|Array|RemoveIndex _array (Variables|Default|GetSpawn%20Index))
    (Variables|/6ga_training/medic/body/body2.body2_C|Setmedic_spawn _returnvalue self))
  (Utilities|Array|Clear _array)
  (bind _returnvalue_2 (Utilities|Time|SetTimerbyEvent (delegate Custom|timer) 3e+02)))

(event Custom|timer
  (CallFunction|DestroyTargets)
  (Actor|Tick|SetActorTickEnabled false))

(event Custom|reset
  (CallFunction|DestroyTargets)
  (Variables|Default|Setbodies 0)
  (Utilities|Time|ClearandInvalidateTimerbyHandle (stale Custom|Spawn%20Body _returnvalue_2))
  (Actor|Tick|SetActorTickEnabled false))

(event Custom|destroy_targets
  (Utilities|FlowControl|Sequence
    (:then_0
      (bind _outactors (Actor|GetAllActorsOfClass "/6ga_training/medic/body/body2.body2_C"))
      (for _array_element _outactors
        (Actor|DestroyActor _array_element)))
    (:then_1
      (bind _outactors_2 (Actor|GetAllActorsOfClass "/6ga_training/medic/body/crouch_BP.crouch_BP_C"))
      (for _array_element_2 _outactors_2
        (Actor|DestroyActor _array_element)))))

(event Custom|decrement
  (bind _result (Math|Integer|DecrementInt (Variables|Default|Getbodies))
    (:%20%20
      (if (== _result 0)
        (Utilities|Time|PauseTimerbyHandle (stale Custom|Spawn%20Body _returnvalue_2))
        (Actor|Tick|SetActorTickEnabled false)))))

(event Custom|update%20time
  (Variables|Default|Settime_remain (Utilities|Time|GetTimerRemainingTimebyHandle (stale Custom|Spawn%20Body _returnvalue_2))))

(event EventTick
  (params (DeltaSeconds :type Float%20%28single-precision%29))
  (CallFunction|UpdateTime))

(fn ConstructionScript)

(fn OnRepTimeRemain
  (if (> (Variables|Default|Gettime_remain) 0.0)
    (Rendering|Components|TextRender|SetTextRenderColor (Variables|Default|Gettime) (Math|Color|MakeColor 0 0 0 255))
    (Rendering|Components|TextRender|SetText (Variables|Default|Gettime) (Utilities|Text|ToText(Float) (Variables|Default|Gettime_remain) "HalfToEven" false true 2 3 2 2))
    (else
      (Rendering|Components|TextRender|SetTextRenderColor (Variables|Default|Gettime) (Math|Color|MakeColor 0 0 255 255))
      (Rendering|Components|TextRender|SetText (Variables|Default|Gettime) (Variables|Default|GetTimes%20up)))))

(fn OnRepBodies
  (Rendering|Components|TextRender|SetText (Variables|Default|Getbodies_num) (Utilities|Text|ToText(Integer) (Variables|Default|Getbodies) false true 1 1)))

(fn BindEventtoAmmoUpdated
  (params (Delegate :type Delegate%20%28by%20ref%29))
  (return false))

(fn CanRearmPawn
  (params (Rearmer :type Pawn%20Object%20Reference))
  (return true))

(fn CanRearmWeapon
  (params (Weapon :type SQ%20Equipable%20Item%20Object%20Reference))
  (return true))

(fn ConsumeAmmo
  (params (AmmoRequired :type Float%20%28single-precision%29))
  (return true))

(fn GetAmmo
  (return 1e+08))

(fn GetRearmNoAmmoString
  (return ""))

(fn GetRearmSuccessString
  (return ""))

(fn GetRearmType
  (return "MainOrEnvironment"))

(fn UnbindEventtoAmmoUpdated
  (params (Delegate :type Delegate%20%28by%20ref%29))
  (return false))