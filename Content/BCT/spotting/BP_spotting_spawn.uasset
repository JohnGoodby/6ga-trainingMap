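; Spawner for a spotting exercise that presents one random German target at a time: a Wehrmacht rifleman, Jagdpanzer IV or Kübelwagen.
; The Randomspawn event destroys the previous target and spawns a new one at the location of one of six arrow components, ignoring arrow rotation.
; It also implements rearm functions as an effectively bottomless ammo source that allows any pawn or weapon to rearm and never depletes.
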(event Custom|Random%20spawn
  (Actor|DestroyActor (stale _returnvalue))
  (bind _returnvalue (Game|SpawnActorfromClass (Utilities|Array|Get(acopy) (Utilities|Array|MakeArray "/Game/PostScriptum/Soldiers/GER/Wehrmacht/BP_PS_GER_Wehrmacht_Rifleman.BP_PS_GER_Wehrmacht_Rifleman_C" "/Game/PostScriptum/Vehicles/Axis/Jagdpanzer_IV/BP_Jagdpanzer_IV.BP_Jagdpanzer_IV_C" "/Game/PostScriptum/Vehicles/Axis/Kubelwagen/BP_Kubelwagen.BP_Kubelwagen_C") (Math|Random|RandomIntegerinRange 0 2)) (Math|Conversions|ToTransform(Vector) (Transformation|GetWorldLocation (Utilities|Array|Get(acopy) (Utilities|Array|MakeArray (Variables|Default|GetArrow) (Variables|Default|GetArrow1) (Variables|Default|GetArrow2) (Variables|Default|GetArrow3) (Variables|Default|GetArrow4) (Variables|Default|GetArrow5)) (Math|Random|RandomIntegerinRange 0 5)))) "AdjustIfPossibleButAlwaysSpawn" 0 0)))

(fn ConstructionScript)

(fn BindEventtoAmmoUpdated
  (params (Delegate :type Delegate%20%28by%20ref%29))
  (return false))

(fn CanRearmPawn
  (params (Rearmer :type Pawn%20Object%20Reference))
  (return true))

(fn CanRearmWeapon
  (params (Weapon :type SQ%20Equipable%20Item%20Object%20Reference))
  (return true))

(fn ConsumeAmmo
  (params (AmmoRequired :type Float%20%28single-precision%29))
  (return true))

(fn GetAmmo
  (return 1e+08))

(fn GetRearmNoAmmoString
  (return ""))

(fn GetRearmSuccessString
  (return ""))

(fn GetRearmType
  (return "MainOrEnvironment"))

(fn UnbindEventtoAmmoUpdated
  (params (Delegate :type Delegate%20%28by%20ref%29))
  (return false))