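; Ambient MG/flak emplacement that fires randomized bursts with muzzle flash and sound while its turret and chassis rotate on timelines.
; Tick drives a Delay-gated Fire event, moving the projectile spawner to the muzzle with slight random angle offsets.
; The server disables it after a timer or when a soldier of the configured team overlaps it.
; The FlakDisabled RepNotify stops tick and destroys both timelines.
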(event Custom|Fire
  (bind _muzzle (Variables|Default|GetMuzzle))
  (bind _returnvalue (Transformation|GetWorldTransform _muzzle))
  (bind (_location _rotation _scale) (Math|Transform|BreakTransform _returnvalue))
  (bind (_roll _pitch _yaw) (Math|Rotator|BreakRotator _rotation))
  ;[1 1 1] Fire Projectiles
  (Utilities|FlowControl|Delay (Variables|Firing|Getprojectiledelay))
  (Variables|Firing|Setburstamount (+ (Variables|Firing|Getburstamount) 1.0))
  (Transformation|SetWorldTransform (Variables|Default|GetSQProjectileSpawner) (Math|Transform|MakeTransform _location (Math|Rotator|MakeRotator _roll (+ _pitch (Math|Random|RandomFloatinRange 1.0 2.0)) (+ _yaw (Math|Random|RandomFloatinRange 1.0 2.0))) _scale) false false)
  (Class|SQProjectileSpawnerComponent|StartFiring (Variables|Default|GetSQProjectileSpawner))
  (Audio|SpawnSoundatLocation (Variables|Firing|GetFiringSound) (Transformation|GetWorldLocation _muzzle) "0, 0, 0" 0.3 0.6 0.0 0 0)
  (Effects|SpawnEmitterAttached "/Game/PostScriptum/FX/Weapons/MuzzleFlashes/Rifles/Muzzleflash_RifleSemiAuto.Muzzleflash_RifleSemiAuto" (Variables|Default|GetMuzzle) "None" "0, 0, 0" "0, 0, 0" "1.000000,1.000000,1.000000" "SnapToTarget"))

(event Custom|ReactivateFlak
  (Variables|Disable|SetFlakDisabled false)
  ;[1 1 1] Turret Rotation
  (Networking|SwitchHasAuthority
    (:Authority
      (Utilities|Time|SetTimerbyEvent (delegate Custom|DisableFlak) (Variables|Disable|GetStopFiringAfterXSeconds))
      (bind _rotation (Timeline|TurretRotation Play)
        (:Update
          (Transformation|SetRelativeRotation (Variables|Default|GetTurret) (Math|Rotator|MakeRotator 0.0 (Variables|Default|GetPitch) (+ _rotation (Variables|Firing|Getstarting%20rotation))) false false)
          (bind _rotation_2 (Timeline|ChassisRotation Play)
            (:Update
              (Transformation|SetRelativeRotation (Variables|Default|GetChassis) (Math|Rotator|MakeRotator 0.0 0.0 (+ _rotation_2 0.0)) false false))))))
    (:Remote
      (if (not (Variables|Disable|GetFlakDisabled))
        (Timeline|TurretRotation Play)))))

(event Custom|DisableFlak
  ;[1 1 1] Disable Flak
  (Variables|Disable|SetFlakDisabled true))

(event Collision|EventActorBeginOverlap
  (params (OtherActor :type Actor%20Object%20Reference))
  ;[1 1 1] Disable when enemy Team near
  (Networking|SwitchHasAuthority
    (:Authority
      (bind _assqsoldier_new (Utilities|Casting|CastToSQSoldierNew OtherActor))
      (if (== (Class|SQSoldier|GetTeam _assqsoldier_new) (Variables|Disable|GetGetsDisabledByTeam))
        (CallFunction|DisableFlak)))))

(event EventTick
  (params (DeltaSeconds :type Float%20%28single-precision%29))
  ;[1 1 1] Make the flak stop firing after x seconds and disable it
  (|CallParentFunction DeltaSeconds)
  (if (not (Variables|Disable|GetFlakDisabled))
    (if (> (Variables|Firing|Getburstamount) (Math|Random|RandomFloatinRange (Variables|Firing|GetMinBurstAmount) (Variables|Firing|GetMaxBurstAmount)))
      (Variables|Firing|Setprojectiledelay (Math|Random|RandomFloatinRange (Variables|Firing|GetMinBurstDelay) (Variables|Firing|GetMaxBurstDelay)))
      (Variables|Firing|Setburstamount 0.0)
      (else
        (Class|SQProjectileSpawnerComponent|StopFiring (Variables|Default|GetSQProjectileSpawner))
        (Variables|Firing|Setprojectiledelay (Variables|Firing|GetFireRate))))
    (CallFunction|Fire)))

(event EventBeginPlay
  ;[1 1 1] Turret Rotation
  (|CallParentFunction)
  (Networking|SwitchHasAuthority
    (:Authority
      (Utilities|Time|SetTimerbyEvent (delegate Custom|DisableFlak) (Variables|Disable|GetStopFiringAfterXSeconds))
      (bind _rotation (Timeline|TurretRotation Play)
        (:Update
          (Transformation|SetRelativeRotation (Variables|Default|GetTurret) (Math|Rotator|MakeRotator 0.0 (Variables|Default|GetPitch) (+ _rotation (Variables|Firing|Getstarting%20rotation))) false false)
          (bind _rotation_2 (Timeline|ChassisRotation Play)
            (:Update
              (Transformation|SetRelativeRotation (Variables|Default|GetChassis) (Math|Rotator|MakeRotator 0.0 0.0 (+ _rotation_2 0.0)) false false))))))
    (:Remote
      (if (not (Variables|Disable|GetFlakDisabled))
        (Timeline|TurretRotation Play)))))

(fn ConstructionScript
  (|CallParentFunction)
  (Components|Sphere|SetSphereRadius (Variables|Default|GetSphere) (Variables|Disable|GetDisableRadius) true))

(fn OnRepFlakDisabled
  (if (Variables|Disable|GetFlakDisabled)
    (CallFunction|DoFlakDisable)))

(fn DoFlakDisable
  (Actor|Tick|SetActorTickEnabled false)
  (Components|DestroyComponent (Variables|Default|GetTurretRotation))
  (Components|DestroyComponent (Variables|Default|GetChassisRotation)))