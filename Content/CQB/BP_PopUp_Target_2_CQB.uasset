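; Pop-up shooting target for a CQB course that drops when damaged enough, either per hit or accumulated.
; It starts up, or rises after a seeded random delay.
; Tick interpolates the target's rotation from IsUp and plays a sound as it nears the down position.
; A qualifying hit clears IsUp, calls CheckTargets on CQB_spawn_BP actors and destroys the target after a short delay, so it never re-raises.
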(event EventBeginPlay
  (bind _output_get (Variables|PopUpTarget|SetbIsUp (Variables|PopUpTarget|GetStartTargetUp)))
  (if _output_get
    (Transformation|SetRelativeRotation (Variables|Default|GetTarget) (Variables|PopUpTarget|GetTargetUpRotation) false false)
    (Variables|PopUpTarget|SetDamageTaken 0.0)
    (Variables|PopUpTarget|SetHasPlayedDroppingSound false)
    (else
      (Transformation|SetRelativeRotation (Variables|Default|GetTarget) (Variables|PopUpTarget|GetTargetDownRotation) false false)
      (Utilities|FlowControl|Delay (Math|Random|RandomFloatinRangefromStream (Variables|PopUpTarget|GetMinTimeToPopUp) (Variables|PopUpTarget|GetMaxTimeToPopUp) (Variables|PopUpTarget|GetRandomStream)))
      (CallFunction|PopUp))))

(event Game|Damage|EventAnyDamage
  (params (Damage :type Float%20%28single-precision%29) (DamageType :type Damage%20Type%20Object%20Reference) (InstigatedBy :type Controller%20Object%20Reference) (DamageCauser :type Actor%20Object%20Reference))
  (bind _mindamagerequiredtodrop (Variables|PopUpTarget|GetMinDamageRequiredToDrop))
  (bind _output_get (Variables|PopUpTarget|SetDamageTaken (+ (Variables|PopUpTarget|GetDamageTaken) Damage)))
  (if (or (and (>= _output_get _mindamagerequiredtodrop) (Variables|PopUpTarget|GetAccumulateDamage)) (and (>= Damage _mindamagerequiredtodrop) (not (Variables|PopUpTarget|GetAccumulateDamage))))
    (Variables|PopUpTarget|SetbIsUp false)
    (bind _outactors (Actor|GetAllActorsOfClass "/6ga_training/CQB/CQB_spawn_BP.CQB_spawn_BP_C"))
    (for _array_element _outactors
      (bind _ascqb_spawn_bp (Utilities|Casting|CastToCQB_spawn_BP _array_element))
      (Default|CheckTargets _ascqb_spawn_bp)
      (Utilities|FlowControl|Delay 0.5)
      (Actor|DestroyActor))))

(event EventTick
  (params (DeltaSeconds :type Float%20%28single-precision%29))
  (bind _target (Variables|Default|GetTarget))
  (bind _targetdownrotation (Variables|PopUpTarget|GetTargetDownRotation))
  (bind _relativerotation (Variables|/Script/Engine.SceneComponent|GetRelativeRotation _target))
  (if (Variables|PopUpTarget|GetbIsUp)
    (Transformation|SetRelativeRotation _target (Math|Interpolation|RInterpTo _relativerotation (Variables|PopUpTarget|GetTargetUpRotation) DeltaSeconds (Variables|PopUpTarget|GetPopUpSpeed)) false false)
    (else
      (Transformation|SetRelativeRotation _target (Math|Interpolation|RInterpTo _relativerotation _targetdownrotation DeltaSeconds (Variables|PopUpTarget|GetDropDownSpeed)) false false)
      (if (not (Variables|PopUpTarget|GetHasPlayedDroppingSound))
        (if (Math|Rotator|Equal(Rotator) _relativerotation _targetdownrotation 1e+01)
          (Audio|SpawnSoundatLocation (Variables|PopUpTarget|GetDropSound) (Transformation|GetActorLocation) "0, 0, 0" 3.0 1.0 0.0 "/Game/Audio/Attenuation/Impacts/Bhits/BhitAttenuation.BhitAttenuation" 0)
          (Variables|PopUpTarget|SetHasPlayedDroppingSound true))))))

(fn ConstructionScript
  (Class|KismetMathLibrary|SeedRandomStream (Variables|PopUpTarget|GetRandomStream)))

(fn PopUp
  (Variables|PopUpTarget|SetbIsUp true)
  (Variables|PopUpTarget|SetDamageTaken 0.0)
  (Variables|PopUpTarget|SetHasPlayedDroppingSound false))