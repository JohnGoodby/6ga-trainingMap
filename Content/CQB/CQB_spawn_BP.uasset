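; CQB training course manager that spawns random pop-up targets and times the run.
; SpawnTargets clears old targets, closes the door, then spawns 8–11 of two target types at unique, randomly picked Arrow markers.
; CheckTargets opens the door when at most one target remains, enabling the finish Box to pause the timer.
; An empty-event timer serves as a stopwatch, its elapsed Time shown on a TextRender through OnRep.
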(event OnComponentBeginOverlap(Box)
  (params (OverlappedComponent :type Primitive%20Component%20Object%20Reference) (OtherActor :type Actor%20Object%20Reference) (OtherComp :type Primitive%20Component%20Object%20Reference) (OtherBodyIndex :type Integer) (bFromSweep :type Boolean) (SweepResult :type Hit%20Result%20Structure%20%28by%20ref%29))
  (if (Variables|Default|GetNoLeft)
    (Utilities|Time|PauseTimerbyHandle (stale Custom|spawn%20targets _returnvalue))
    (Variables|Default|Settime (Class|KismetSystemLibrary|GetTimerElapsedTimeHandle (stale Custom|spawn%20targets _returnvalue)))))

(event Custom|spawn%20targets
  (bind _array (Variables|Default|Getarray))
  (Variables|Default|Settime 0.0)
  (CallFunction|DestroyTargets)
  (Variables|Default|Setdone true)
  (Variables|Default|SetNoLeft false)
  (Rendering|SetVisibility (Variables|Default|GetDoor) true false)
  (Collision|SetCollisionEnabled (Variables|Default|GetDoor) "QueryAndPhysics")
  (Utilities|Time|ClearandInvalidateTimerbyHandle (stale _returnvalue))
  (for _array_element (Utilities|Array|MakeArray (Variables|Default|GetArrow) (Variables|Default|GetArrow1) (Variables|Default|GetArrow2) (Variables|Default|GetArrow3) (Variables|Default|GetArrow4) (Variables|Default|GetArrow5) (Variables|Default|GetArrow6) (Variables|Default|GetArrow7) (Variables|Default|GetArrow8) (Variables|Default|GetArrow9) (Variables|Default|GetArrow10) (Variables|Default|GetArrow11) (Variables|Default|GetArrow12) (Variables|Default|GetArrow13) (Variables|Default|GetArrow14) (Variables|Default|GetArrow15) (Variables|Default|GetArrow16) (Variables|Default|GetArrow17) (Variables|Default|GetArrow18) (Variables|Default|GetArrow19))
    (Utilities|Array|Add (Variables|Default|Getarray) _array_element))
  (for _index (range 0 (Math|Random|RandomIntegerinRange 8 11))
    (Math|Integer|IncrementInt (Variables|Default|GetNumberSpawned)
      (:%20%20
        (Variables|Default|SetspawnIndex (Math|Random|RandomInteger (Utilities|Array|Length _array)))
        (Game|SpawnActorfromClass (Utilities|Array|Get(acopy) (Utilities|Array|MakeArray "/6ga_training/CQB/BP_PopUp_Target_2_CQB.BP_PopUp_Target_2_CQB_C" "/6ga_training/CQB/BP_PopUp_Target_CQB.BP_PopUp_Target_CQB_C") (Math|Random|RandomIntegerinRange 0 1)) (Transformation|GetWorldTransform (Utilities|Array|Get(acopy) _array (Variables|Default|GetspawnIndex))) "AdjustIfPossibleButAlwaysSpawn" 0 0)
        (Utilities|Array|RemoveIndex _array (Variables|Default|GetspawnIndex))
        (bind _returnvalue (Utilities|Time|SetTimerbyEvent (delegate Custom|CustomEvent_0) 3e+02)))))
  (Utilities|Array|Clear _array))

(event Custom|destroy_targets
  (Utilities|FlowControl|Sequence
    (:then_0
      (bind _outactors (Actor|GetAllActorsOfClass "/6ga_training/CQB/BP_PopUp_Target_CQB.BP_PopUp_Target_CQB_C"))
      (for _array_element _outactors
        (Actor|DestroyActor _array_element)))
    (:then_1
      (bind _outactors_2 (Actor|GetAllActorsOfClass "/6ga_training/CQB/BP_PopUp_Target_2_CQB.BP_PopUp_Target_2_CQB_C"))
      (for _array_element_2 _outactors_2
        (Actor|DestroyActor _array_element)))))

(event Custom|check%20targets
  (Utilities|FlowControl|Sequence
    (:then_0
      (bind _outactors (Actor|GetAllActorsOfClass "/6ga_training/CQB/BP_PopUp_Target_CQB.BP_PopUp_Target_CQB_C")))
    (:then_1
      (bind _outactors_2 (Actor|GetAllActorsOfClass "/6ga_training/CQB/BP_PopUp_Target_2_CQB.BP_PopUp_Target_2_CQB_C"))
      (if (not (> (+ (Utilities|Array|Length _outactors) (Utilities|Array|Length _outactors_2)) 1))
        (Rendering|SetVisibility (Variables|Default|GetDoor) false false)
        (Collision|SetCollisionEnabled (Variables|Default|GetDoor) "NoCollision")
        (Variables|Default|SetNoLeft true)))))

(event Custom|CustomEvent_0)

(event EventBPonUsed
  (params (User :type Controller%20Object%20Reference))
  (Default|Used (Variables|Default|GetBP_ContextSensitiveUsableComponent) User))

(event EventBPStopUsed
  (params (User :type Controller%20Object%20Reference))
  (Default|StopUsed (Variables|Default|GetBP_ContextSensitiveUsableComponent) User))

(fn ConstructionScript)

(fn OnRepTime
  (Rendering|Components|TextRender|SetText (Variables|Default|GetTextRender1) (Utilities|Text|ToText(Float) (Variables|Default|Gettime) "HalfToEven" false true 2 3 2 2)))

(fn GetInterfaceTeam
  (return 0))

(fn GetTeamId
  (return 0))

(fn GetUsableData
  (return ""))