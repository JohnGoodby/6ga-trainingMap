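; Moving training target with a Wehrmacht helmet that slides along world X by a set distance on a timeline.
; Damage above a threshold triggers impact particles plus either a body-hit sound or a physics helmet launch with headshot feedback, chosen by the FirstHit flag.
; After a short delay it resets position; with authority, it increments score on Moving_targets_BP, calls Repeat and destroys itself.
; An unhit run also calls Repeat and destroys itself.
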(event Game|Damage|EventAnyDamage
  (params (Damage :type Float%20%28single-precision%29) (DamageType :type Damage%20Type%20Object%20Reference) (InstigatedBy :type Controller%20Object%20Reference) (DamageCauser :type Actor%20Object%20Reference))
  (if (> Damage 1e+01)
    (Variables|Default|Setdamaged true)
    (if (Variables|Default|GetFirstHit)
      (CallFunction|Sounds)
      (else
        (CallFunction|HelmetFly)))
    (CallFunction|Effects)
    (Variables|Default|SetFirstHit true)
    (Utilities|FlowControl|Delay 0.3)
    (Transformation|SetWorldLocation (Variables|Default|GetDefaultSceneRoot) (Variables|Default|GetInitialLocation) false false)
    (Variables|Default|Setdamaged false)
    (bind _asmoving_targets_bp (Utilities|Casting|CastToMoving_targets_BP (Variables|Default|Getactor)))
    (Networking|SwitchHasAuthority
      (:Authority
        (Default|ScoreIncrement _asmoving_targets_bp)
        (Default|Repeat _asmoving_targets_bp)
        (Actor|DestroyActor))
      (:Remote
        (Development|PrintString "not authority")))))

(event EventBeginPlay
  (Variables|Default|SetInitialLocation (Transformation|GetWorldLocation (Variables|Default|GetDefaultSceneRoot)))
  (bind _alpha (Timeline|fast PlayFromStart)
    (:Update
      (CallFunction|Movements _alpha))
    (:Finished
      (bind _asmoving_targets_bp (Utilities|Casting|CastToMoving_targets_BP (Variables|Default|Getactor)))
      (Default|Repeat _asmoving_targets_bp)
      (Actor|DestroyActor))))

(fn ConstructionScript)

(fn Effects
  (bind _pfxorigin1 (Variables|Default|GetPFxOrigin1))
  (bind _pfxorigin2 (Variables|Default|GetPFxOrigin2))
  (Effects|SpawnEmitteratLocation (Variables|Default|GetParticleEffect) (Transformation|GetWorldLocation _pfxorigin1) (Transformation|GetWorldRotation _pfxorigin1))
  (Effects|SpawnEmitteratLocation (Variables|Default|GetParticleEffect) (Transformation|GetWorldLocation _pfxorigin2) (Transformation|GetWorldRotation _pfxorigin2)))

(fn HelmetFly
  (bind _sm_werhmacht_helmet (Variables|Default|GetSM_Werhmacht_Helmet))
  (bind _sk_werhmacht_m40 (Variables|Default|GetSK_Werhmacht_M40))
  (bind _returnvalue (Transformation|GetWorldLocation _sk_werhmacht_m40))
  (Physics|SetSimulatePhysics (Variables|Default|GetSM_Werhmacht_Helmet) true)
  (Class|PrimitiveComponent|AddForceatLocation _sm_werhmacht_helmet (* (Math|Vector|GetUpVector _sm_werhmacht_helmet) "-80000.000000, 0,100000.000000") _returnvalue "None")
  (Audio|SpawnSoundatLocation "/Game/PostScriptum/Audio/Impacts/Bullets/Body/Feedback/Headshot_feedback_cue.Headshot_feedback_cue" _returnvalue "0, 0, 0" 5.0 1.0 0.0 0 0))

(fn Sounds
  (Audio|SpawnSoundatLocation "/Game/PostScriptum/Audio/Impacts/Bullets/Body/Feedback/Bullet_body_impact_feedback_light_cue.Bullet_body_impact_feedback_light_cue" (Transformation|GetWorldLocation (Variables|Default|Getlogmid01)) "0, 0, 0" 5.0 1.0 0.0 0 0))

(fn Movements
  (params (Alpha :type Float%20%28single-precision%29))
  (Transformation|SetWorldLocation (Variables|Default|GetDefaultSceneRoot) (Math|Vector|Lerp(Vector) (Variables|Default|GetInitialLocation) (+ (Variables|Default|GetInitialLocation) (Math|Vector|MakeVector (Variables|Default|GetDistance) 0.0 0.0)) Alpha) false false))